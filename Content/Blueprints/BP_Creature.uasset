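; BP_Creature is an AI enemy that hunts the player by following a scent trail and ends the game on contact.
; It repeatedly asks BP_ScentGrid for the strongest neighboring scent location and moves there with AIMoveTo, re-evaluating whenever a move ends.
; Without a scent, it wanders to random navigable points nearby.
; Overlapping the player with KillRadius disables input, shows the game-over widget and halts the creature.
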(event `self.ReceiveBeginPlay`
  (bind _outactors (`GameplayStatics.GetAllActorsOfClass` "/Game/Blueprints/BP_ScentGrid.BP_ScentGrid_C"))
  (set `self.ScentGridRef` (`|GetArrayItem` _outactors))
  (`self.UpdateCreaturePath`))

(event `UpdateCreaturePath`
  (bind _returnvalue (`self.K2_GetActorLocation`))
  (if (not (`self.IsGameOver`))
    (bind _bestlocation__ (`/Game/Blueprints/BP_ScentGrid.GetStrongestNeighborLocation` (`self.ScentGridRef`) _returnvalue))
    (if (!= _bestlocation__ (0.0 0.0 0.0))
      (set `self.IsWandering` false)
      (`|AIMoveTo` self _bestlocation__ null 50.0
        (:`OnSuccess`
          _)
        (:`OnFail`
          _))
      (`self.UpdateCreaturePath`)
      (elif (not (`self.IsWandering`))
        (set `self.IsWandering` true)
        (bind _randomlocation (`NavigationSystemV1.K2_GetRandomLocationInNavigableRadius` _returnvalue 1000.0 null null))
        (`|AIMoveTo` self _randomlocation null 50.0
          (:`OnSuccess`
            _)
          (:`OnFail`
            _))
        (set `self.IsWandering` false)
        (`self.UpdateCreaturePath`)))))

(event `self.KillRadius.OnComponentBeginOverlap`
  (params (OverlappedComponent :type "PrimitiveComponent Object Reference") (OtherActor :type "Actor Object Reference") (OtherComp :type "PrimitiveComponent Object Reference") (OtherBodyIndex :type Integer) (bFromSweep :type Boolean) (SweepResult :type "HitResult Structure (by ref)"))
  (bind _asbp_third_person_character (cast `/Game/ThirdPerson/Blueprints/BP_ThirdPersonCharacter` OtherActor))
  (`self.DisableInput` _asbp_third_person_character (`GameplayStatics.GetPlayerController` 0))
  (bind _returnvalue (`|CreateWidget` "/Game/UI/WBP_GameOver.WBP_GameOver_C"))
  (`UserWidget.AddToViewport` _returnvalue 0)
  (set `self.IsGameOver` true)
  (`MovementComponent.StopMovementImmediately` (`self.CharacterMovement`)))

(fn `UserConstructionScript`)