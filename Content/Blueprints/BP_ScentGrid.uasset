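; BP_ScentGrid is a world-placed scent map that stores scent strength in a flat 2D cell array anchored at the actor's location.
; AddScentAtPosition deposits scent into neighboring cells, scaling radius by amount with distance falloff, while a looping timer decays every cell.
; GetStrongestNeighborLocation searches nearby cells for markedly stronger scent and returns that world position, or zero if none qualifies.
; A second timer draws a blue-to-red debug heatmap.
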(event `self.ReceiveBeginPlay`
  (set `self.GridOrigin` (`self.K2_GetActorLocation`))
  (for _ (range (* (`self.GridHeight`) (`self.GridWidth`)))
    (`KismetArrayLibrary.Array_Add` (`self.ScentValues`)))
  (`KismetSystemLibrary.K2_SetTimerDelegate` (delegate `ApplyDecay`) 1.0 true)
  (`KismetSystemLibrary.K2_SetTimerDelegate` (delegate `DrawHeatmap`) 0.5 true))

(event `ApplyDecay`
  (for (_array_element _array_index) (`self.ScentValues`)
    (`KismetArrayLibrary.Array_Set` (`self.ScentValues`) _array_index (* _array_element (`self.DecayRate`)))))

(event `DrawHeatmap`
  (for (_array_element _array_index) (`self.ScentValues`)
    (if (> _array_element 0.1)
      (`KismetSystemLibrary.DrawDebugBox` (`self.GridIndexToWorldPos` _array_index) (45.0 45.0 2.0) (`KismetMathLibrary.LinearColorLerp` (struct :`B` 1.0 :`A` 1.0) (struct :`R` 1.0 :`A` 1.0) _array_element) (struct) 0.55 2.0))))

(fn `AddScentAtPosition`
  (params (`WorldPos ` :type "Vector Structure") (`ScentAmount ` :type "Float (double-precision)"))
  (locals (CenterX :type Integer :default 0) (CenterY :type Integer))
  (bind _index (`self.WorldToGridIndex` `WorldPos `))
  (set `local.CenterX` (mod _index (`self.GridWidth`)))
  (set `local.CenterY` (/ _index (`self.GridWidth`)))
  (bind _output_get (set `self.LocalRadius` (`KismetMathLibrary.FTrunc` (`KismetMathLibrary.MapRangeClamped` `ScentAmount ` 0.0 100.0 1.0 5.0))))
  (bind _returnvalue (* _output_get -1))
  (for _index_2 (range _returnvalue (+ _output_get 1))
    (for _index_3 (range _returnvalue (+ _output_get 1))
      (`self.SpreadToNeighbor` (+ (`local.CenterX`) _index_3) (+ (`local.CenterY`) _index_2) (/ `ScentAmount ` (+ (`KismetMathLibrary.VSize2D` (`KismetMathLibrary.MakeVector2D` (`KismetMathLibrary.Conv_IntToDouble` _index_3) (`KismetMathLibrary.Conv_IntToDouble` _index_2))) 1.0))))
    (return)))

(fn `DrawDebugHeatmap`
  (for (_array_element _array_index) (`self.ScentValues`)
    (`KismetSystemLibrary.DrawDebugBox` (+ (`KismetMathLibrary.MakeVector` (* (mod _array_index (`self.GridWidth`)) (`self.CellSize`)) (* (/ _array_index (`self.GridWidth`)) (`self.CellSize`))) (`self.GridOrigin`)) (50.0 50.0 1.0) (`KismetMathLibrary.LinearColorLerp` (make `LinearColor` 0.0 0.0 0.0 1.0) (make `LinearColor` 1.0) _array_element) (struct) 0.0 2.0)))

(fn `GetStrongestNeighborLocation`
  (params (`WorldPos ` :type "Vector Structure"))
  (returns (`BestLocation  ` :type "Vector Structure"))
  (bind _index (`self.WorldToGridIndex` `WorldPos `))
  (set `self.BestValue` 0.1)
  (set `self.BestLocation` (0.0 0.0 0.0))
  (for _index_2 (range -3 4)
    (for _index_3 (range -3 4)
      (bind _returnvalue (+ (mod _index (`self.GridWidth`)) _index_2))
      (bind _returnvalue_2 (+ (/ _index (`self.GridWidth`)) _index_3))
      (if (and (>= _returnvalue 0) (< _returnvalue (`self.GridWidth`)) (>= _returnvalue_2 0) (< _returnvalue_2 (`self.GridHeight`)))
        (if (not (and (== _index_2 0) (== _index_3 0)))
          (bind _returnvalue_3 (+ (* _returnvalue_2 (`self.GridWidth`)) _returnvalue))
          (bind _output (`|GetArrayItem` (`self.ScentValues`) _returnvalue_3))
          (if (> _output (+ (`self.BestValue`) 2.0))
            (set `self.BestValue` _output)
            (set `self.BestLocation` (`self.GridIndexToWorldPos` _returnvalue_3)))))))
  (return (`self.BestLocation`)))

(fn `GridIndexToWorldPos`
  (params (Index :type Integer))
  (returns (CenterLocation :type "Vector Structure"))
  (return (+ (+ (`KismetMathLibrary.MakeVector` (* (mod Index (`self.GridWidth`)) (`self.CellSize`)) (* (/ Index (`self.GridWidth`)) (`self.CellSize`))) (`self.GridOrigin`)) (50.0 50.0 10.0))))

(fn `SpreadToNeighbor`
  (params (TargetX :type Integer) (TargetY :type Integer) (ScentAmount :type "Float (double-precision)"))
  (bind _scentvalues (`self.ScentValues`))
  (bind _returnvalue (+ (* TargetY (`self.GridWidth`)) TargetX))
  (if (and (>= TargetX 0) (< TargetX (`self.GridWidth`)) (>= TargetY 0) (< TargetY (`self.GridHeight`)))
    (`KismetArrayLibrary.Array_Set` _scentvalues _returnvalue (+ (`|GetArrayItem` _scentvalues _returnvalue) ScentAmount))))

(fn `UserConstructionScript`)

(fn `WorldToGridIndex`
  (params (WorldPos :type "Vector Structure"))
  (returns (Index :type Integer))
  (return (+ (`KismetMathLibrary.FFloor` (/ (.x (- WorldPos (`self.GridOrigin`))) (`self.CellSize`))) (* (`KismetMathLibrary.FFloor` (/ (.y (- WorldPos (`self.GridOrigin`))) (`self.CellSize`))) (`self.GridWidth`)))))